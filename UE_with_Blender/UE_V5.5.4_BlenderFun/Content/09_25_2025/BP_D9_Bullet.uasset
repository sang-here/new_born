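; BP_D9_Bullet is a physics projectile that destroys BP_D8_Enemy actors it overlaps, then itself.
; On BeginPlay it applies an impulse to its Sphere along the Arrow1 forward vector of each BP_D9_FirstAndThirdPersonCharacter found in the world.
; A function-name timer calls its DestroyActor wrapper to remove the bullet after a short lifetime.
; An equivalent launch function targeting the D8 character remains but is not called here.
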(event OnComponentBeginOverlap(Sphere)
  (params (OverlappedComponent :type Primitive%20Component%20Object%20Reference) (OtherActor :type Actor%20Object%20Reference) (OtherComp :type Primitive%20Component%20Object%20Reference) (OtherBodyIndex :type Integer) (bFromSweep :type Boolean) (SweepResult :type Hit%20Result%20Structure%20%28by%20ref%29))
  (bind _asbp_d8_enemy (Utilities|Casting|CastToBP_D8_Enemy OtherActor))
  (Actor|DestroyActor _asbp_d8_enemy)
  (Development|PrintString "Enemy got a shot")
  (Actor|DestroyActor))

(event EventBeginPlay
  (D9|D9ShootItfromFirstPerson)
  (Utilities|Time|SetTimerbyFunctionName 0 "DestroyActor" 5.0))

(fn ConstructionScript)

(fn DestroyActor
  (Actor|DestroyActor))

(fn D8ShootItfromFirstPerson
  (bind _outactors (Actor|GetAllActorsOfClass "/Game/09_24_2025/BP_D8_FirstAndThirdPersonCharacter.BP_D8_FirstAndThirdPersonCharacter_C"))
  (for _array_element _outactors
    (Physics|AddImpulse (Variables|Default|GetSphere) (* (Math|Vector|GetForwardVector (Variables|/Game/09_24_2025/BP_D8_FirstAndThirdPersonCharacter.BP_D8_FirstAndThirdPersonCharacter_C|GetArrow1 _array_element)) 5e+03) "None" false)))

(fn D9ShootItfromFirstPerson
  (bind _outactors (Actor|GetAllActorsOfClass "/Game/09_25_2025/BP_D9_FirstAndThirdPersonCharacter.BP_D9_FirstAndThirdPersonCharacter_C"))
  (for _array_element _outactors
    (Physics|AddImpulse (Variables|Default|GetSphere) (* (Math|Vector|GetForwardVector (Variables|/Game/09_25_2025/BP_D9_FirstAndThirdPersonCharacter.BP_D9_FirstAndThirdPersonCharacter_C|GetArrow1 _array_element)) 5e+03) "None" false)))