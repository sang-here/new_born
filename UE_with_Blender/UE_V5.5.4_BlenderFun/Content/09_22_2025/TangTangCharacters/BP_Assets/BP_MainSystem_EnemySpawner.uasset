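; BP_MainSystem_EnemySpawner is a spawner actor that fills a ring with BP_Enemy actors.
; Every Tick it spawns 36 enemies, with no timer or limit, at ten-degree steps on a 1000-unit circle around the world origin.
; Sine and cosine of the loop index give each X and Y position.
; An unconnected construction-script loop would place static mesh components in a smaller ring the same way.
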(event EventBeginPlay)

(event EventTick
  (params (DeltaSeconds :type Float%20%28single-precision%29))
  (for _index (range 0 35)
    ;[0.15 0.15 0.15 0.5] 원 그리기 0 ~ 360
    ; sine의 첫 = 0, cos의 첫 = 1
    (Game|SpawnActorfromClass "/Game/09_22_2025/TangTangCharacters/Anim/BP_Enemy.BP_Enemy_C" (Math|Transform|MakeTransform (Math|Vector|MakeVector (* (Math|Trig|Sin(Degrees) (Math|Conversions|ToFloat(Integer) (* _index 10))) 1e+03) (* (Math|Trig|Cos(Degrees) (Math|Conversions|ToFloat(Integer) (* _index 10))) 1e+03) 0.0) "0, 0, 0" "1.000000,1.000000,1.000000") "Undefined" "MultiplyWithRoot" 0 0)))

(fn ConstructionScript
  ;[0.15 0.15 0.15 0.5] Test
)