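; BP_D8_EnemySpawnerUFO is a spawner that creates a BP_D8_Enemy at its Arrow's world transform every tick and stores it in an array.
; On BeginPlay, two pairs of ping-pong timelines sweep the Arrow's yaw back and forth and bob it up and down, varying the spawn transform.
; A timeline-based cleanup that destroys stored enemies in order is present but never runs, so this Blueprint removes none.
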(event EventTick
  (params (DeltaSeconds :type Float%20%28single-precision%29))
  (bind _enemyinstance (D8|SpawnEnemy))
  (Utilities|Array|Add (Variables|Default|GetEnemySpawnedArray) _enemyinstance))

(event EventBeginPlay
  (Utilities|FlowControl|Sequence
    (:then_0
      ;[0.15 0.15 0.15 0.5] Spawner Rotater / Maybe not good or pretty codes, but it works at least
      (Timeline|Timeline Play
        (:Update
          (if (>= (.yaw (Variables|/Script/Engine.SceneComponent|GetRelativeRotation (Variables|Default|GetArrow))) 6e+01)
            (Development|PrintString "Max")
            (Utilities|FlowControl|Sequence
              (:then_0
                (Timeline|Timeline Stop))
              (:then_1
                (Timeline|Timeline_0 Play
                  (:Update
                    (if (<= (.yaw (Variables|/Script/Engine.SceneComponent|GetRelativeRotation (Variables|Default|GetArrow))) -6e+01)
                      (Development|PrintString "Minimum")
                      (Utilities|FlowControl|Sequence
                        (:then_0
                          (Timeline|Timeline_0 Stop))
                        (:then_1
                          (Timeline|Timeline Play)))
                      (else
                        (Transformation|AddRelativeRotation (Variables|Default|GetArrow) "0.000000,-0.500000,0.000000" false false))))
                  (:Finished
                    (Timeline|Timeline_0 PlayFromStart)))))
            (else
              (Transformation|AddRelativeRotation (Variables|Default|GetArrow) "0.000000,0.500000,0.000000" false false))))
        (:Finished
          (Timeline|Timeline PlayFromStart))))
    (:then_1
      ;[0.15 0.15 0.15 0.5] Spawner UpDownMover / Maybe not good or pretty codes, but it works at least
      (Timeline|Timeline_1 Play
        (:Update
          (if (>= (.z (Variables|/Script/Engine.SceneComponent|GetRelativeLocation (Variables|Default|GetArrow))) 1e+02)
            (Utilities|FlowControl|Sequence
              (:then_0
                (Timeline|Timeline_1 Stop))
              (:then_1
                (Timeline|Timeline_2 Play
                  (:Update
                    (if (<= (.z (Variables|/Script/Engine.SceneComponent|GetRelativeLocation (Variables|Default|GetArrow))) 0.0)
                      (Utilities|FlowControl|Sequence
                        (:then_0
                          (Timeline|Timeline_2 Stop))
                        (:then_1
                          (Timeline|Timeline_1 Play)))
                      (else
                        (Transformation|AddRelativeLocation (Variables|Default|GetArrow) "0.000000,0.000000,-1.000000" false false))))
                  (:Finished
                    (Timeline|Timeline_2 PlayFromStart)))))
            (else
              (Transformation|AddRelativeLocation (Variables|Default|GetArrow) "0.000000,0.000000,1.000000" false false))))
        (:Finished
          (Timeline|Timeline_1 PlayFromStart))))))

(fn ConstructionScript)

(fn SpawnEnemy
  (bind _returnvalue (Game|SpawnActorfromClass "/Game/09_24_2025/BP_D8_Enemy.BP_D8_Enemy_C" (Transformation|GetWorldTransform (Variables|Default|GetArrow)) "Undefined" "MultiplyWithRoot" 0 0))
  (return _returnvalue))