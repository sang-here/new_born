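; BP_D8_Enemy is an enemy character that is launched from D8 spawners, then chases the player.
; On BeginPlay its mesh simulates physics and takes an impulse along the arrow of every BP_D8_Spawn.
; Two seconds later physics stops, the capsule moves to the mesh and the mesh is realigned.
; AI MoveTo then targets the player, reissued on a five-second delay; mesh hits print the other component's name.
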(event OnComponentHit(Mesh)
  (params (HitComponent :type Primitive%20Component%20Object%20Reference) (OtherActor :type Actor%20Object%20Reference) (OtherComp :type Primitive%20Component%20Object%20Reference) (NormalImpulse :type Vector :default "0, 0, 0") (Hit :type Hit%20Result%20Structure%20%28by%20ref%29))
  (Development|PrintString (Utilities|GetDisplayName OtherComp)))

(event EventBeginPlay
  (Physics|SetSimulatePhysics (Variables|Character|GetMesh) true)
  (D8|ShootMeshfromtheD8Spawner)
  (Utilities|FlowControl|Delay 2.0)
  (Physics|SetSimulatePhysics (Variables|Character|GetMesh) false)
  (Transformation|SetWorldTransform (Variables|Collision|GetCapsuleComponent) (Math|Transform|MakeTransform (.location (Transformation|GetWorldTransform (Variables|Character|GetMesh))) "0, 0, 0" "1.000000,1.000000,1.000000") false false)
  (Transformation|SetRelativeTransform (Variables|Character|GetMesh) (Math|Transform|MakeTransform (Math|Vector|MakeVector 0.0 0.0 -89.0) (Math|Rotator|MakeRotator 0.0 0.0 2.7e+02) "1.000000,1.000000,1.000000") false false)
  (AI|AIMoveTo self "0, 0, 0" (Game|Player|GetPlayerPawn 0) 5.0 false :!label _label
    (:then
      _)
    (:OnFail
      _))
  (Utilities|FlowControl|Delay 5.0)
  (goto _label))

(fn ConstructionScript)

(fn ShootMeshfromtheD8Spawner
  (bind _outactors (Actor|GetAllActorsOfClass "/Game/09_24_2025/BP_D8_Spawn.BP_D8_Spawn_C"))
  (for _array_element _outactors
    (Physics|AddImpulse (Variables|Character|GetMesh) (* (Math|Vector|GetForwardVector (Variables|/Game/09_24_2025/BP_D8_Spawn.BP_D8_Spawn_C|GetArrow _array_element)) 2e+04) "None" false)))