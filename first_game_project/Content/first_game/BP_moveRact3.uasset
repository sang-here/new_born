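; Moving actor Blueprint that shuttles its Pantteigi component back and forth along an L-shaped path (ㄴ) in the local X-Z plane.
; Each Tick switches on a direction enum, NewVar, and adds a fixed relative offset, so speed depends on frame rate.
; Relative-location limits advance the state from Right to Up, then Down and Left to retrace the path, looping endlessly.
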(event EventTick
  (params (DeltaSeconds :type Float%20%28single-precision%29))
  ;[0.15 0.15 0.15 0.5] ㄴ을 그리며 움직이는 코드
  (switch Utilities|FlowControl|Switch|SwitchonENUM_move_type_3 (Variables|Default|GetNewVar)
    (:NewEnumerator0
      (Transformation|AddRelativeLocation (Variables|Default|Getpantteigi) (Math|Vector|MakeVector 5.0 0.0 0.0) false false)
      (if (>= (.x (Variables|/Script/Engine.SceneComponent|GetRelativeLocation (Variables|Default|Getpantteigi))) 2.5e+02)
        (Variables|Default|SetNewVar "NewEnumerator1")))
    (:NewEnumerator1
      (Transformation|AddRelativeLocation (Variables|Default|Getpantteigi) (Math|Vector|MakeVector 0.0 0.0 5.0) false false)
      (if (>= (.z (Variables|/Script/Engine.SceneComponent|GetRelativeLocation (Variables|Default|Getpantteigi))) 2.5e+02)
        (Variables|Default|SetNewVar "NewEnumerator2")))
    (:NewEnumerator2
      (Transformation|AddRelativeLocation (Variables|Default|Getpantteigi) (Math|Vector|MakeVector 0.0 0.0 -5.0) false false)
      (if (<= (.z (Variables|/Script/Engine.SceneComponent|GetRelativeLocation (Variables|Default|Getpantteigi))) 0.0)
        (Variables|Default|SetNewVar "NewEnumerator3")))
    (:NewEnumerator3
      (Transformation|AddRelativeLocation (Variables|Default|Getpantteigi) (Math|Vector|MakeVector -5.0 0.0 -0.0) false false)
      (if (<= (.x (Variables|/Script/Engine.SceneComponent|GetRelativeLocation (Variables|Default|Getpantteigi))) 0.0)
        (Variables|Default|SetNewVar "NewEnumerator0")))))

(fn ConstructionScript)